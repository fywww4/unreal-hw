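; Tanuki NPC Blueprint whose Paper2D sprite slides into place when play begins.
; BeginPlay caches the sprite's relative location as the end point, then fires the SlideIn event.
; SlideIn plays a timeline at double rate, lerping the sprite from SlideStartPos to that cached position.
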(event `self.ReceiveBeginPlay`
  (set `self.Sprite Default pos` (`SceneComponent.RelativeLocation` (`self.Paper Sprite`)))
  (`self.SlideIn`))

(event `SlideIn`
  (`TimelineComponent.SetPlayRate` (`self.SlideInAnim`) 2.0)
  (bind (_direction _alpha) (`Timeline|SlideInAnim` :!via `PlayFromStart`)
    (:`Update`
      (`SceneComponent.K2_SetRelativeLocation` (`self.Paper Sprite`) (`KismetMathLibrary.VLerp` (`self.Slide Start pos`) (`self.Sprite Default pos`) _alpha) false false))))

(fn `UserConstructionScript`)